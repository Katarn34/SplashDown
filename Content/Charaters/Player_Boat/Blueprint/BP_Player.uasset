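; Player boat pawn that moves in flying mode and fishes for treasure with a cable-linked grappling hook.
; Grab detaches the BP_Hook child actor as a projectile, HookHit homes it back, and overlap on return reattaches it and destroys the treasure.
; Looping timers refresh the aim vector and toggle splash VFX and engine sound from velocity.
; Per-player high-score save macros exist, but their event-graph logic is never run.
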(event OnComponentBeginOverlap(HookCollision)
  (params (OverlappedComponent :type Primitive%20Component%20Object%20Reference) (OtherActor :type Actor%20Object%20Reference) (OtherComp :type Primitive%20Component%20Object%20Reference) (OtherBodyIndex :type Integer) (bFromSweep :type Boolean) (SweepResult :type Hit%20Result%20Structure%20%28by%20ref%29))
  (bind _hook_ref (Variables|Default|GetHook%20Ref))
  ;[1 1 1] Hook Return
  (if (== OtherActor (.AsBP%20Hook (Utilities|Casting|CastToBP_Hook (Variables|/Script/Engine.ChildActorComponent|GetChildActor (Variables|Default|GetChildActor)))))
    (if (Variables|System|Getis%20Grappling)
      (Variables|System|Setis%20Grappling false)
      (Variables|/Script/Engine.ProjectileMovementComponent|SetbIsHomingProjectile (Variables|/Game/_GameManager/GameObjects/Hook/Blueprint/BP_Hook.BP_Hook_C|GetProjectileMovement (Variables|Default|GetHook%20Ref)) false)
      (Variables|/Script/Engine.MovementComponent|SetVelocity (Variables|/Game/_GameManager/GameObjects/Hook/Blueprint/BP_Hook.BP_Hook_C|GetProjectileMovement (Variables|Default|GetHook%20Ref)) "0, 0, 0")
      (Transformation|SetActorLocationAndRotation (Variables|Default|GetHook%20Ref) (Transformation|GetWorldLocation (Variables|Default|GetHookReturnPoint)) (Variables|Default|GetHookRotation) false true)
      (Variables|System|SetHook%20Coming%20Back%20? false)
      (Default|DestroyTreasure _hook_ref)
      (Transformation|AttachComponentToComponent _hook_ref (Variables|Default|GetHookReturnPoint) "None" "KeepWorld" "KeepWorld" "KeepWorld" true)
      (Audio|Components|Audio|Stop (stale Custom|Hook%20Hit _returnvalue))
      (Audio|PlaySound2D "/Game/Sound_Sam/SD/Boat/SC_Hameçon_réenclenche.SC_Hameçon_réenclenche" 1.0 1.0 0.0 0 0)
      (Rendering|SetVisibility (Variables|Default|GetWidget) true false)
      (Variables|Sounds|SetHook%20Going%20Sound false)
      (Variables|Sounds|SetHook%20Come%20Back%20Sound false)
      (Variables|/Game/_GameManager/GameObjects/Hook/Blueprint/BP_Hook.BP_Hook_C|SetHook%20Come%20Back%20Sound (Variables|Default|GetHook%20Ref) false)
      (Variables|System|SetIsOnBoat%20? true)
      (Utilities|Array|Clear (Variables|/Game/_GameManager/GameObjects/Hook/Blueprint/BP_Hook.BP_Hook_C|GetTreasure%20Score (Variables|Default|GetHook%20Ref))))))

(event Custom|Timer0
  (bind _returnvalue (Game|GetPlayerController 0))
  ;[1 1 1] Timer
  (Input|SetInputModeUIOnly _returnvalue 0 "DoNotLock" false)
  (Variables|/Script/Engine.PlayerController|SetbShowMouseCursor _returnvalue true)
  (Utilities|FlowControl|Delay 1.8e+02)
  (Audio|PlaySound2D "/Game/Sound_Sam/SD/Timer/SC_timer_1tick.SC_timer_1tick" 1.0 1.0 0.0 0 0)
  (Utilities|FlowControl|Delay 15.0)
  (Audio|PlaySound2D "/Game/Sound_Sam/SD/Timer/SC_timer_2ticks.SC_timer_2ticks" 1.0 1.0 0.0 0 0)
  (Utilities|FlowControl|Delay 15.0)
  (Audio|PlaySound2D "/Game/Sound_Sam/SD/Timer/SC_timer_3ticks.SC_timer_3ticks" 1.0 1.0 0.0 0 0))

(event Custom|Boat%20Moving%20VFX%20&%20Sound
  ;[1 1 1] VFX Splash Boat
  (bind _event (|VFXSplashboat)))

(event Custom|Hook%20Hit
  (bind _childactor (Variables|Default|GetChildActor))
  (bind _sound_hook_begin (Variables|Sounds|GetSound%20Hook%20Begin))
  (bind _childactor_2 (Variables|/Script/Engine.ChildActorComponent|GetChildActor _childactor))
  (bind _asbp_hook (Utilities|Casting|CastToBP_Hook _childactor_2))
  ;[1 1 1] Hook Hitting
  (Components|Activation|Deactivate (Variables|/Game/_GameManager/GameObjects/Hook/Blueprint/BP_Hook.BP_Hook_C|GetTrail _asbp_hook))
  (Components|Activation|Deactivate (Variables|/Game/_GameManager/GameObjects/Hook/Blueprint/BP_Hook.BP_Hook_C|GetVFXTrail (Variables|Default|GetHook%20Ref)))
  (Collision|SetCollisionResponsetoChannel (Variables|/Game/_GameManager/GameObjects/Hook/Blueprint/BP_Hook.BP_Hook_C|GetGrab%20Collision _asbp_hook) "ECC_Vehicle" "ECR_Ignore")
  (Collision|SetCollisionResponsetoChannel (Variables|/Game/_GameManager/GameObjects/Hook/Blueprint/BP_Hook.BP_Hook_C|GetHook _asbp_hook) "ECC_WorldDynamic" "ECR_Overlap")
  (Utilities|IsValid _sound_hook_begin
    (:Is%20Valid
      (Audio|Components|Audio|Stop _sound_hook_begin))
    (:Is%20Not%20Valid
      _))
  (Variables|/Script/Engine.ProjectileMovementComponent|SetbIsHomingProjectile (Variables|/Game/_GameManager/GameObjects/Hook/Blueprint/BP_Hook.BP_Hook_C|GetProjectileMovement (Variables|Default|GetHook%20Ref)) true)
  (Variables|/Script/Engine.ProjectileMovementComponent|SetHomingTargetComponent (Variables|/Game/_GameManager/GameObjects/Hook/Blueprint/BP_Hook.BP_Hook_C|GetProjectileMovement (Variables|Default|GetHook%20Ref)) (Variables|Default|GetHookReturnPoint))
  (bind _velocity (|HookComebackSpeed))
  (Variables|/Script/Engine.MovementComponent|SetVelocity (Variables|/Game/_GameManager/GameObjects/Hook/Blueprint/BP_Hook.BP_Hook_C|GetProjectileMovement (Variables|Default|GetHook%20Ref)) (* _velocity -1e+01))
  (Variables|System|SetHook%20Coming%20Back%20? true)
  (if (not (Variables|Sounds|GetHook%20Come%20Back%20Sound))
    (Variables|Sounds|SetHook%20Come%20Back%20Sound true)
    (bind _returnvalue (Audio|SpawnSound2D "/Game/Sound_Sam/SD/Boat/SC_Hamecon_retour_Cue.SC_Hamecon_retour_Cue" 1.0 1.0 0.0 0))))

(event Custom|Grab
  (bind _hook_ref (Variables|Default|GetHook%20Ref))
  (bind _vfxtrail (Variables|/Game/_GameManager/GameObjects/Hook/Blueprint/BP_Hook.BP_Hook_C|GetVFXTrail _hook_ref))
  ;[1 1 1] Grapplin Mechanic - Changing Velocity
  (Variables|System|SetIsOnBoat%20? false)
  (Variables|System|Setis%20Grappling true)
  (Rendering|SetVisibility (Variables|Default|GetWidget) false false)
  (Transformation|DetachFromActor (Variables|/Script/Engine.ChildActorComponent|GetChildActor (Variables|Default|GetChildActor)) "KeepWorld" "KeepWorld" "KeepWorld")
  (Collision|SetCollisionResponsetoChannel (Variables|/Game/_GameManager/GameObjects/Hook/Blueprint/BP_Hook.BP_Hook_C|GetGrab%20Collision (Variables|Default|GetHook%20Ref)) "ECC_Vehicle" "ECR_Overlap")
  (Variables|Default|SetHookRotation (Transformation|GetActorRotation (Variables|Default|GetHook%20Ref)))
  (Variables|/Script/Engine.MovementComponent|SetVelocity (Variables|/Game/_GameManager/GameObjects/Hook/Blueprint/BP_Hook.BP_Hook_C|GetProjectileMovement (Variables|Default|GetHook%20Ref)) (* (Variables|Default|GetHookForwardVector) (Variables|Default|GetHookSpeed)))
  (Components|Activation|Activate _vfxtrail false)
  ;;[1 0.02652 0] Provisoire
  (Niagara|ResetSystem _vfxtrail)
  (Components|Activation|Activate (Variables|/Game/_GameManager/GameObjects/Hook/Blueprint/BP_Hook.BP_Hook_C|GetTrail _hook_ref) false)
  (if (not (Variables|Sounds|GetHook%20Going%20Sound))
    (Variables|Sounds|SetHook%20Going%20Sound true)
    (Variables|Sounds|SetCan%20Delete%20Sound%20? true)
    (bind _returnvalue (Audio|SpawnSound2D "/Game/Sound_Sam/SD/Boat/SC_Hamecon_aller_Cue.SC_Hamecon_aller_Cue" 1.0 1.0 0.0 0))
    (bind _output_get (Variables|Sounds|SetSound%20Hook%20Begin _returnvalue))))

(event Custom|ForwardVector
  ;[1 1 1] HookForwardVector Calculation
  (Variables|Default|SetHookForwardVector (|ForwardCalculator)))

(event Custom|Game%20Finished
  ;[1 1 1] Stop fishing sounds when finished
  (Utilities|FlowControl|Sequence
    (:then_0
      (Utilities|IsValid (stale Custom|Grab _output_get)
        (:Is%20Valid
          (Audio|Components|Audio|Stop (stale Custom|Grab _output_get)))))
    (:then_1
      (Utilities|IsValid (stale Custom|Hook%20Hit _returnvalue)
        (:Is%20Valid
          (Audio|Components|Audio|Stop (stale Custom|Hook%20Hit _returnvalue)))))))

(event Custom|Hit%20Times%20Integer
  ;[1 1 1] Increment Hit Times Big Treasure
  (Variables|Default|SetHit%20Times (+ (Variables|Default|GetHit%20Times) 1)))

(event Custom|Set%20The%20Score)

(event Custom|End%20Game
  (bind _widget (Variables|Default|GetWidget))
  (Widget|RemovefromParent (UserInterface|GetWidget _widget))
  (Components|DestroyComponent _widget))

(event EventBeginPlay
  (bind _childactor (Variables|Default|GetChildActor))
  (bind _childactor_2 (Variables|/Script/Engine.ChildActorComponent|GetChildActor _childactor))
  (bind _asbp_hook (Utilities|Casting|CastToBP_Hook _childactor_2))
  (Utilities|Time|SetTimerbyEvent (delegate Custom|Boat%20Moving%20VFX%20&%20Sound) 0.05 true)
  (Utilities|Time|SetTimerbyEvent (stale Custom|Boat%20Moving%20VFX%20&%20Sound _event) 0.05 true)
  ;[1 1 1] Setting BP_Hook as child of PB_player
  (Actor|SetOwner (Variables|/Script/Engine.ChildActorComponent|GetChildActor (Variables|Default|GetChildActor)) self)
  (Utilities|Time|SetTimerbyEvent (delegate Custom|ForwardVector) 0.05 true)
  ;[1 1 1] Attaching Cable to BP_Hook
  (Variables|Default|SetHook%20Ref _asbp_hook)
  (Class|CableComponent|SetAttachEndtoComponent (Variables|Default|GetCable) (Variables|/Game/_GameManager/GameObjects/Hook/Blueprint/BP_Hook.BP_Hook_C|GetStartPoint _asbp_hook) "None")
  (Pawn|Components|CharacterMovement|SetMovementMode (Variables|Character|GetCharacterMovement) "MOVE_Flying" 0))

(event EventTick
  (params (DeltaSeconds :type Float%20%28single-precision%29))
  (Transformation|AddLocalRotation (Variables|Default|GetHéliceOrange) "2.500000,0.000000,0.000000" false false)
  (Transformation|AddLocalRotation (Variables|Default|GetPériOrange) "0.000000,2.000000,0.000000" false false)
  (Transformation|AddLocalRotation (Variables|Default|GetPériVert) "0.000000,2.000000,0.000000" false false)
  (Transformation|AddLocalRotation (Variables|Default|GetHéliceVert) "2.500000,0.000000,0.000000" false false))

(fn ConstructionScript)

(event Custom|Spawning%20Boat%20Sounds
  (if (or (Variables|VFX|GetVFX%20Splash%20Ahead) (Variables|VFX|GetVFX%20Splash%20Behind))
    (if (not (Variables|Sounds|GetBoat%20Sounds))
      (bind _returnvalue (Audio|SpawnSound2D "/Game/Sound_Sam/SD/Boat/SC_Bateau_qui_avance_4.SC_Bateau_qui_avance_4" 1.0 1.0 0.0 0))
      (Variables|Sounds|SetBoat%20Sounds true))
    (elif (Variables|Sounds|GetBoat%20Sounds)
      (Variables|Sounds|SetBoat%20Sounds false)
      (Audio|Components|Audio|Stop _returnvalue))))
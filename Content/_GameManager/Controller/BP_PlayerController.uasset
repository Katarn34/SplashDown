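; Player controller for a treasure-hook game with two scored players, handling Enhanced Input for movement, hook and pause menu.
; Grab fires or hits the pawn's BP_Hook, or becomes a button-mash on a big treasure, driving feedback, sound and spam count.
; Each mash runs IncrBigT, which adds points to player one or two by the pawn's GetAllActorsOfClass index.
; The B key cuts the match timer to seconds.
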(event Input|EnhancedActionEvents|EnhancedInputActionIA_Move
  (params (ActionValue :type Vector%202D%20Structure) (ElapsedSeconds :type Float%20%28double-precision%29) (TriggeredSeconds :type Float%20%28double-precision%29) (InputAction :type Input%20Action%20Object%20Reference :default "/Game/_GameManager/Input/InputAction/IA_Move.IA_Move"))
  (bind _returnvalue (Pawn|GetControlledPawn))
  ;[1 1 1] Movement  Left/Right
  (Pawn|Input|AddMovementInput _returnvalue (Transformation|GetActorForwardVector _returnvalue) (.x ActionValue) true))

(event Input|EnhancedActionEvents|EnhancedInputActionIA_Options
  (params (ActionValue :type Boolean) (ElapsedSeconds :type Float%20%28double-precision%29) (TriggeredSeconds :type Float%20%28double-precision%29) (InputAction :type Input%20Action%20Object%20Reference :default "/Game/_GameManager/Input/InputAction/IA_Options.IA_Options"))
  ;[1 1 1] Menu Pause
  (Game|SetGamePaused true)
  (Input|SetInputModeUIOnly self 0 "DoNotLock" false)
  (bind _returnvalue (UserInterface|CreateWidget "/Game/UI-UX/Menus/WBP_Settings.WBP_Settings_C"))
  (UserInterface|Viewport|AddtoViewport _returnvalue 0))

(event Input|EnhancedActionEvents|EnhancedInputActionIA_Grab
  (params (ActionValue :type Boolean) (ElapsedSeconds :type Float%20%28double-precision%29) (TriggeredSeconds :type Float%20%28double-precision%29) (InputAction :type Input%20Action%20Object%20Reference :default "/Game/_GameManager/Input/InputAction/IA_Grab.IA_Grab"))
  ;[1 1 1] Hook Input
  (bind _asbp_player (Utilities|Casting|CastToBP_Player (Pawn|GetControlledPawn)))
  (bind _output_get (Variables|Default|SetControlled%20Pawn%20Ref _asbp_player))
  (bind _output_get_2 (Variables|Default|SetHook%20controlled%20Ref (.AsBP%20Hook (Utilities|Casting|CastToBP_Hook (Variables|/Script/Engine.ChildActorComponent|GetChildActor (Variables|/Game/Charaters/Player_Boat/Blueprint/BP_Player.BP_Player_C|GetChildActor _output_get))))))
  (if (Variables|/Game/_GameManager/GameObjects/Hook/Blueprint/BP_Hook.BP_Hook_C|GetBig%20Treasure%20Hit _output_get_2)
    ;[1 1 1] Spam
    (Default|HitTimesInteger (Variables|Default|GetControlled%20Pawn%20Ref))
    (Utilities|IsValid (Variables|Default|GetSC%20Spam)
      (:Is%20Valid
        (Audio|Components|Audio|Stop (Variables|Default|GetSC%20Spam))
        (bind _returnvalue (Audio|SpawnSound2D "/Game/Sound_Sam/SD/SpamClicVF/SC_spamgold_VF.SC_spamgold_VF" 1.0 1.0 0.0 0))
        (Variables|Default|SetSC%20Spam _returnvalue))
      (:Is%20Not%20Valid
        (bind _returnvalue_2 (Audio|SpawnSound2D "/Game/Sound_Sam/SD/SpamClicVF/SC_spamgold_VF.SC_spamgold_VF" 1.0 1.0 0.0 0))
        (Variables|Default|SetSC%20Spam _returnvalue_2)))
    (bind _returnvalue_3 (Actor|GetActorOfClass "/Game/_GameManager/GameObjects/Big_Treasure/Blueprint/BP_BigTreasure.BP_BigTreasure_C"))
    (Variables|/Game/_GameManager/GameObjects/Big_Treasure/Blueprint/BP_BigTreasure.BP_BigTreasure_C|SetCan%20go%20Next%20Animation%20? _returnvalue_3 false)
    (Default|BigTreasureFeedback _returnvalue_3)
    (bind _ashud_spam (Utilities|Casting|CastToHUD_Spam (UserInterface|GetWidget (Variables|/Game/_GameManager/GameObjects/Hook/Blueprint/BP_Hook.BP_Hook_C|GetHUD_Spam (Variables|Default|GetHook%20controlled%20Ref)))))
    (Variables|/Game/UI-UX/HUD/HUD_Spam.HUD_Spam_C|SetCount _ashud_spam (+ (Variables|/Game/UI-UX/HUD/HUD_Spam.HUD_Spam_C|GetCount _ashud_spam) 1.0))
    (Utilities|FlowControl|Sequence
      (:then_0
        ;[1 1 1] Incr Score by 5 for each hit on the Big Treasure
        (|IncrBigT))
      (:then_1
        (Components|Activation|Activate (Variables|/Game/_GameManager/GameObjects/Hook/Blueprint/BP_Hook.BP_Hook_C|GetTreasureHit (Variables|Default|GetHook%20controlled%20Ref)) false)
        (Utilities|FlowControl|Delay 0.1)
        (Components|Activation|Deactivate (Variables|/Game/_GameManager/GameObjects/Hook/Blueprint/BP_Hook.BP_Hook_C|GetTreasureHit (Variables|Default|GetHook%20controlled%20Ref)))))
    (elif (Variables|/Game/Charaters/Player_Boat/Blueprint/BP_Player.BP_Player_C|Getis%20Grappling (Variables|Default|GetControlled%20Pawn%20Ref))
      (if (not (Variables|/Game/Charaters/Player_Boat/Blueprint/BP_Player.BP_Player_C|GetHook%20Coming%20Back%20? (Variables|Default|GetControlled%20Pawn%20Ref)))
        (Default|HookHit (Variables|Default|GetControlled%20Pawn%20Ref)))
      (else
        (Default|Grab (Variables|Default|GetControlled%20Pawn%20Ref))))))

(event EventBeginPlay
  (bind _returnvalue (PlayerController|LocalPlayerSubsystems|GetEnhancedInputLocalPlayerSubsystem))
  ;[1 1 1] Add Mapping input to player
  (Utilities|IsValid _returnvalue
    (:Is%20Valid
      (Input|AddMappingContext _returnvalue "/Game/_GameManager/Input/IMC_Player.IMC_Player" 0 "(bIgnoreAllPressedKeysUntilRelease=True,bForceImmediately=False,bNotifyUserSettings=False)"))))

(event Input|KeyboardEvents|B
  (params (Key :type Key%20Structure :default "None"))
  (:Pressed
    (bind _foundwidgets (Widget|GetAllWidgetsOfClass "/Game/UI-UX/HUD/HUD_Timer.HUD_Timer_C" true))
    (for _array_element _foundwidgets
      (Variables|/Game/UI-UX/HUD/HUD_Timer.HUD_Timer_C|SetMinutes _array_element 0)
      (Variables|/Game/UI-UX/HUD/HUD_Timer.HUD_Timer_C|SetSeconds _array_element 5))))

(fn ConstructionScript)
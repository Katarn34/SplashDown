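; BP_Treasure3 is a physics-driven treasure object that gets a launch impulse at BeginPlay and bounces on contact.
; On hit it ignores BP_Hook, kicks up and sideways off BP_Treasure1 based on its Y velocity, and otherwise gets a tiny impulse meant to maintain height.
; It also sets the ProjectileMovement initial speed from TreasureSpeed, and its construction script fixes the actor's rotation.
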(event EventBeginPlay
  ;[1 1 1] Base Impulse
  (Variables|/Script/Engine.ProjectileMovementComponent|SetInitialSpeed (Variables|Default|GetProjectileMovement) (Variables|Default|GetTreasure%20Speed))
  (Physics|AddImpulse (Variables|Default|GetTreasure) (Variables|Default|GetFirst%20Impulse) "None" true))

(event Collision|EventHit
  (params (MyComp :type Primitive%20Component%20Object%20Reference) (Other :type Actor%20Object%20Reference) (OtherComp :type Primitive%20Component%20Object%20Reference) (bSelfMoved :type Boolean) (HitLocation :type Vector :default "0, 0, 0") (HitNormal :type Vector :default "0, 0, 0") (NormalImpulse :type Vector :default "0, 0, 0") (Hit :type Hit%20Result%20Structure%20%28by%20ref%29))
  ;[1 1 1] What is the treasure touching verification
  (bind _asbp_hook (Utilities|Casting|CastToBP_Hook Other)
    (:then
      _)
    (:CastFailed
      _))
  (if (not (== _asbp_hook Other))
    (bind _asbp_treasure (Utilities|Casting|CastToBP_Treasure1 Other)
      (:then
        _)
      (:CastFailed
        _))
    (if (== Other _asbp_treasure)
      ;[1 1 1] Add impulse on touching itself on linear velocity check
      (bind _returnvalue (Physics|GetPhysicsLinearVelocity (Variables|Default|GetTreasure) "None"))
      (if (<= (.y _returnvalue) 1.0)
        (Physics|AddImpulse (Variables|Default|GetTreasure) "0.000000,-200.000000,75.000000" "None" true)
        (else
          (Physics|AddImpulse (Variables|Default|GetTreasure) "0.000000,200.000000,75.000000" "None" true)))
      (else
        ;[1 1 1] Add Impulse to maintain height
        (Physics|AddImpulse (Variables|Default|GetTreasure) "0.000000,1.000000,1.000000" "None" false)))))

(fn ConstructionScript
  (Transformation|SetActorRotation "0.000000,90.000000,0.000000"))
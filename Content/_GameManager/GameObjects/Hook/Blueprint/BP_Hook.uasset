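; Player-owned grappling hook for a two-player treasure-grabbing game, which swings between roll limits on timers until the player fires it.
; Overlaps attach treasures or urchins (Ursin) to the hook and trigger its return; DestroyTreasure later destroys them, adjusting that player's score and popup widgets.
; A big treasure instead pins the hook and shows a spam prompt; the owner reaching 20 hits wins bonus points and ends the contest.
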(event OnComponentBeginOverlap(GrabCollision)
  (params (OverlappedComponent :type Primitive%20Component%20Object%20Reference) (OtherActor :type Actor%20Object%20Reference) (OtherComp :type Primitive%20Component%20Object%20Reference) (OtherBodyIndex :type Integer) (bFromSweep :type Boolean) (SweepResult :type Hit%20Result%20Structure%20%28by%20ref%29))
  ;[1 1 1] Hook Collision System : Identify what is hit and execute the code which is related
  (Variables|Default|SetGrabbed%20Actor OtherActor)
  (bind _asbp_player (Utilities|Casting|CastToBP_Player (Components|GetOwner)))
  (Variables|Default|SetPlayer%20Ref _asbp_player)
  (if (not (Variables|/Game/Charaters/Player_Boat/Blueprint/BP_Player.BP_Player_C|GetIsOnBoat%20? _asbp_player))
    (bind _returnvalue (Actor|GetActorOfClass "/Game/_GameManager/GameObjects/Big_Treasure/Blueprint/BP_BigTreasure.BP_BigTreasure_C"))
    (if (== _returnvalue (Variables|Default|GetGrabbed%20Actor))
      (|BigTreasureIsHit
        (:OutputPin
          (|UrsinIsHit :!label _label
            (:false2
              (|TreasureIsHit)))))
      (else
        (goto _label False)))))

(event OnProjectileBounce(ProjectileMovement)
  (params (ImpactResult :type Hit%20Result%20Structure%20%28by%20ref%29) (ImpactVelocity :type Vector%20%28by%20ref%29 :default "0, 0, 0"))
  ;[1 1 1] On Hitting, return to it's position
  (if (not (Variables|Default|GetBig%20Treasure%20Hit))
    (bind _asbp_player (Utilities|Casting|CastToBP_Player (Components|GetOwner)))
    (Default|HookHit _asbp_player)
    (Components|Activation|Activate (Variables|Default|GetBaseHit) false)
    (if (Variables|Sounds|GetHook%20Come%20Back%20Sound)
      _
      (else
        (Variables|Sounds|SetHook%20Come%20Back%20Sound true)
        (Audio|PlaySound2D "/Game/Sound_Sam/SD/Collision/SC_Collision_neutre.SC_Collision_neutre" 1.0 1.0 0.0 0 0)))
    (Utilities|FlowControl|Delay 0.5)
    (Components|Activation|Deactivate (Variables|Default|GetBaseHit))))

(event Custom|Number%20of%20Hits%20?
  ;[1 1 1] Big Treasure 20 Times Hit System
  (if (Variables|Default|GetBig%20Treasure%20Hit)
    (bind _asbp_player (Utilities|Casting|CastToBP_Player (Components|GetOwner)))
    (Variables|Default|SetAs%20BP%20Player _asbp_player)
    (if (== (Variables|/Game/Charaters/Player_Boat/Blueprint/BP_Player.BP_Player_C|GetHit%20Times _asbp_player) 20)
      (Variables|Default|SetWinner true)
      (bind _returnvalue (Actor|GetActorOfClass "/Game/_GameManager/GameObjects/Big_Treasure/Blueprint/BP_BigTreasure.BP_BigTreasure_C"))
      (Default|BigTreasureFinished _returnvalue)
      (bind _outactors (Actor|GetAllActorsOfClass "/Game/Charaters/Player_Boat/Blueprint/BP_Player.BP_Player_C"))
      (for _array_element _outactors
        (Variables|/Game/Charaters/Player_Boat/Blueprint/BP_Player.BP_Player_C|SetHit%20Times _array_element 0)))))

(event Custom|Hook%20Reset
  ;[1 1 1] Conditions
  (|AttachActorVerification))

(event Custom|End%20Game
  (Components|DestroyComponent (Variables|Default|GetScoreIncrr)))

(event Custom|Cycle
  (bind _returnvalue (Transformation|GetActorRotation))
  (bind _returnvalue_2 (Transformation|GetActorRotation))
  ;[1 1 1] Rotation Cycle
  (if (and (<= (.roll _returnvalue_2) -105.0) (>= (.roll _returnvalue_2) -1.2e+02))
    (Variables|System|SetStopRotation%201 true)
    (else
      (Variables|System|SetStopRotation%202 false)
      (if (and (<= (.roll _returnvalue) 1.2e+02) (>= (.roll _returnvalue) 105.0))
        (Variables|System|SetStopRotation%202 true)
        (else
          (Variables|System|SetStopRotation%201 false))))))

(event Custom|Hit%20Treasure%20/%20Ursin
  ;[1 1 1] Conditions
  (Variables|/Game/Charaters/Player_Boat/Blueprint/BP_Player.BP_Player_C|SetHook%20Coming%20Back%20? (Variables|Default|GetPlayer%20Ref) false)
  (Default|HookHit (Variables|Default|GetPlayer%20Ref)))

(event Custom|Destroy%20Treasure
  (bind _returnvalue (Components|GetOwner))
  ;[1 1 1] Destroy Treasure Touch
  (|DestroyActors
    (:true
      (bind _outactors (Actor|GetAllActorsOfClass "/Game/Charaters/Player_Boat/Blueprint/BP_Player.BP_Player_C"))
      (if (== (Utilities|Array|Get(acopy) _outactors) _returnvalue)
        (Variables|Default|SetTreasure%20Touch false)
        (bind _foundwidgets (Widget|GetAllWidgetsOfClass "/Game/UI-UX/HUD/HUD_Score.HUD_Score_C" true))
        (|AddScoreP1 _foundwidgets :!pinned true ; AddScore P1
          (:Treasure
            (|ShowHUDIncr/DecrP1 :!label _label))
          (:Ursin
            (goto _label execute)))
        (elif (== (Utilities|Array|Get(acopy) _outactors 1) _returnvalue)
          (Variables|Default|SetTreasure%20Touch false)
          (bind _foundwidgets_2 (Widget|GetAllWidgetsOfClass "/Game/UI-UX/HUD/HUD_Score.HUD_Score_C" true))
          (|AddScoreP2 _foundwidgets_2 :!pinned true ; AddScore P2
            (:Treasure
              (|ShowHUDIncr/DecrP2 :!label _label_2))
            (:Ursin
              (goto _label_2 execute))))))))

(event Custom|Rotating%20Hook
  (bind _hook (Variables|Default|GetHook))
  ;[1 1 1] Rotation Movement
  (bind _asbp_player (Utilities|Casting|CastToBP_Player (Components|GetOwner)))
  (if (not (Variables|/Game/Charaters/Player_Boat/Blueprint/BP_Player.BP_Player_C|Getis%20Grappling _asbp_player))
    (switch int (Variables|System|GetSelection)
      (:0
        (if (Variables|System|GetStopRotation%201)
          (Variables|System|SetSelection 1)
          (else
            (Transformation|AddWorldRotation _hook (Math|Rotator|MakeRotator (* (Variables|RotationRate|GetRotation%20Left) 0.013) 0.0 0.0) false false))))
      (:1
        (if (Variables|System|GetStopRotation%202)
          (Variables|System|SetSelection 0)
          (else
            (Transformation|AddWorldRotation _hook (Math|Rotator|MakeRotator (* 0.013 (Variables|RotationRate|GetRotation%20Right)) 0.0 0.0) false false)))))))

(event Custom|Big%20Treasure%20Hook%20Finished
  (bind _scoreincrr (Variables|Default|GetScoreIncrr))
  (bind _hud_spam (Variables|Default|GetHUD_Spam))
  ;[1 1 1] Big Treasure 20 Times Hit System
  (if (Variables|Default|GetBig%20Treasure%20Hit)
    (Variables|Default|SetBig%20Treasure%20Hit false)
    (bind _returnvalue (Actor|GetActorOfClass "/Game/_GameManager/GameObjects/Big_Treasure/Blueprint/BP_SpawnBigTreasure.BP_SpawnBigTreasure_C"))
    (Transformation|DetachFromActor "KeepWorld" "KeepWorld" "KeepWorld")
    (bind _asbp_player (Utilities|Casting|CastToBP_Player (Components|GetOwner)))
    (Variables|/Game/Charaters/Player_Boat/Blueprint/BP_Player.BP_Player_C|SetHook%20Coming%20Back%20? _asbp_player false)
    (Transformation|AttachComponentToComponent (Variables|/Game/Charaters/Player_Boat/Blueprint/BP_Player.BP_Player_C|GetHookReturnPoint _asbp_player) "None" "KeepWorld" "KeepWorld" "KeepWorld" true)
    (Variables|/Game/_GameManager/GameObjects/Big_Treasure/Blueprint/BP_SpawnBigTreasure.BP_SpawnBigTreasure_C|SetBig%20Treasure%20Appear _returnvalue false)
    (Collision|SetCollisionEnabled (Variables|Default|GetGrab%20Collision) "QueryOnly")
    (Variables|/Script/Engine.MovementComponent|SetVelocity (Variables|Default|GetProjectileMovement) "1.000000,0.000000,0.000000")
    (Default|HookHit _asbp_player)
    (Utilities|FlowControl|Sequence
      (:then_0
        (bind _foundwidgets (Widget|GetAllWidgetsOfClass "/Game/UI-UX/HUD/HUD_Spam.HUD_Spam_C" false))
        (for _array_element _foundwidgets
          (Default|Spam _array_element)
          (Transformation|AttachComponentToComponent _hud_spam (Variables|Default|GetHook) "None" "KeepWorld" "KeepWorld" "KeepWorld" true)
          (Rendering|SetVisibility _hud_spam false false)
          (Audio|PlaySound2D "/Game/Sound_Sam/SD/Score/SC_score_gros_tresor.SC_score_gros_tresor" 1.0 1.0 0.0 0 0)))
      (:then_1
        (if (Variables|Default|GetWinner)
          (bind _foundwidgets_2 (Widget|GetAllWidgetsOfClass "/Game/UI-UX/HUD/HUD_Score.HUD_Score_C" true))
          (|AddScore_2_2_2_2 _foundwidgets_2 ; AddScore
            (:then
              _)
            (:out
              _))
          (bind _foundwidgets_3 (Widget|GetAllWidgetsOfClass "/Game/UI-UX/HUD/HUD_IncrementTreasure.HUD_IncrementTreasure_C" false))
          (Variables|/Game/UI-UX/HUD/HUD_IncrementTreasure.HUD_IncrementTreasure_C|SetIncrrTreasure (Utilities|Array|Get(acopy) _foundwidgets_3) 50)
          (Rendering|SetVisibility _scoreincrr true false)
          (Utilities|FlowControl|Delay 1.0)
          (Rendering|SetVisibility _scoreincrr false false)
          (Variables|Default|SetWinner false)
          (bind _foundwidgets_4 (Widget|GetAllWidgetsOfClass "/Game/UI-UX/HUD/HUD_IncrementTreasure.HUD_IncrementTreasure_C" false))
          (for _array_element_2 _foundwidgets_4
            (Variables|/Game/UI-UX/HUD/HUD_IncrementTreasure.HUD_IncrementTreasure_C|SetIncrrTreasure _array_element_2 0)))))))

(event EventBeginPlay
  (Utilities|Time|SetTimerbyEvent (delegate Custom|Rotating%20Hook) 0.01 true)
  (bind _foundwidgets (Widget|GetAllWidgetsOfClass "/Game/UI-UX/HUD/HUD_IncrementTreasure.HUD_IncrementTreasure_C" false))
  (Variables|WBPRef|SetWBP%20Increment%20P1 (Utilities|Array|Get(acopy) _foundwidgets))
  (Variables|WBPRef|SetWBP%20Increment%20P2 (Utilities|Array|Get(acopy) _foundwidgets 1))
  (bind _foundwidgets_2 (Widget|GetAllWidgetsOfClass "/Game/UI-UX/HUD/HUD_DecrementUrsins.HUD_DecrementUrsins_C" false))
  (Variables|WBPRef|SetWBP%20Decrement%20P1 (Utilities|Array|Get(acopy) _foundwidgets_2))
  (Variables|WBPRef|SetWBP%20Decrement%20P2 (Utilities|Array|Get(acopy) _foundwidgets_2 1))
  (Utilities|Time|SetTimerbyEvent (delegate Custom|Cycle) 0.06 true)
  ;[1 1 1] Big Treasure 20 Times Hit System
  (Utilities|Time|SetTimerbyEvent (delegate Custom|Number%20of%20Hits%20?) 0.1 true))

(fn ConstructionScript)
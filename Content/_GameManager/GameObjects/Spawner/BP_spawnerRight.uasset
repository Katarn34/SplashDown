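; Right-side spawner that creates BP_Treasure1 at its Box on a looping timer until the HUD_Timer countdown reaches zero.
; Each tick reads the remaining time to choose one of three phases, each with its own random odds for speed tiers.
; Medium and fast rolls set speed on an existing treasure, not the spawned one, and flag BP_Hook.
; Slow rolls spawn nothing because their speed and spawn nodes are disconnected.
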(event Custom|Spawn
  ;[1 1 1] First Minute
  (bind _foundwidgets (Widget|GetAllWidgetsOfClass "/Game/UI-UX/HUD/HUD_Timer.HUD_Timer_C" true))
  (if (>= (Variables|/Game/UI-UX/HUD/HUD_Timer.HUD_Timer_C|GetMinutes (Utilities|Array|Get(acopy) _foundwidgets)) 2)
    (if (and (== (Variables|/Game/UI-UX/HUD/HUD_Timer.HUD_Timer_C|GetMinutes (Utilities|Array|Get(acopy) _foundwidgets)) 2) (<= (Variables|/Game/UI-UX/HUD/HUD_Timer.HUD_Timer_C|GetSeconds (Utilities|Array|Get(acopy) _foundwidgets)) 30))
      ;[1 1 1] Second minute
      (bind _foundwidgets_2 (Widget|GetAllWidgetsOfClass "/Game/UI-UX/HUD/HUD_Timer.HUD_Timer_C" true :!label _label))
      (if (>= (Variables|/Game/UI-UX/HUD/HUD_Timer.HUD_Timer_C|GetMinutes (Utilities|Array|Get(acopy) _foundwidgets_2)) 1)
        (if (and (== (Variables|/Game/UI-UX/HUD/HUD_Timer.HUD_Timer_C|GetMinutes (Utilities|Array|Get(acopy) _foundwidgets_2)) 1) (<= (Variables|/Game/UI-UX/HUD/HUD_Timer.HUD_Timer_C|GetSeconds (Utilities|Array|Get(acopy) _foundwidgets_2)) 30))
          ;[1 1 1] Last Minute
          (bind _foundwidgets_3 (Widget|GetAllWidgetsOfClass "/Game/UI-UX/HUD/HUD_Timer.HUD_Timer_C" true :!label _label_2))
          (if (>= (Variables|/Game/UI-UX/HUD/HUD_Timer.HUD_Timer_C|GetMinutes (Utilities|Array|Get(acopy) _foundwidgets_3)) 0)
            (if (not (and (== (Variables|/Game/UI-UX/HUD/HUD_Timer.HUD_Timer_C|GetMinutes (Utilities|Array|Get(acopy) _foundwidgets_3)) 0) (== (Variables|/Game/UI-UX/HUD/HUD_Timer.HUD_Timer_C|GetSeconds (Utilities|Array|Get(acopy) _foundwidgets_3)) 0)))
              (Variables|Default|SetPercent (Math|Random|RandomFloat))
              (if (and (>= (Variables|Default|GetPercent) 0.0) (<= (Variables|Default|GetPercent) 0.3))
                (bind _returnvalue (Actor|GetActorOfClass "/Game/_GameManager/GameObjects/Treasure/Blueprint/BP_Treasure1.BP_Treasure1_C"))
                (Variables|/Game/_GameManager/GameObjects/Treasure/Blueprint/BP_Treasure1.BP_Treasure1_C|SetTreasure%20Speed _returnvalue 8e+02)
                (Game|SpawnActorfromClass "/Game/_GameManager/GameObjects/Treasure/Blueprint/BP_Treasure1.BP_Treasure1_C" (Transformation|GetWorldTransform (Variables|Default|GetBox)) "Undefined" "MultiplyWithRoot" 0 0)
                (bind _returnvalue_2 (Actor|GetActorOfClass "/Game/_GameManager/GameObjects/Hook/Blueprint/BP_Hook.BP_Hook_C"))
                (Variables|/Game/_GameManager/GameObjects/Hook/Blueprint/BP_Hook.BP_Hook_C|SetIsMiddle? _returnvalue_2 true)
                (elif (and (>= (Variables|Default|GetPercent) 0.4) (<= (Variables|Default|GetPercent) 1.0))
                  (bind _returnvalue_3 (Actor|GetActorOfClass "/Game/_GameManager/GameObjects/Treasure/Blueprint/BP_Treasure1.BP_Treasure1_C"))
                  (Variables|/Game/_GameManager/GameObjects/Treasure/Blueprint/BP_Treasure1.BP_Treasure1_C|SetTreasure%20Speed _returnvalue_3 1e+03)
                  (Game|SpawnActorfromClass "/Game/_GameManager/GameObjects/Treasure/Blueprint/BP_Treasure1.BP_Treasure1_C" (Transformation|GetWorldTransform (Variables|Default|GetBox)) "Undefined" "MultiplyWithRoot" 0 0)
                  (bind _returnvalue_4 (Actor|GetActorOfClass "/Game/_GameManager/GameObjects/Hook/Blueprint/BP_Hook.BP_Hook_C"))
                  (Variables|/Game/_GameManager/GameObjects/Hook/Blueprint/BP_Hook.BP_Hook_C|SetIsFast? _returnvalue_4 true)
                  (elif (and (>= (Variables|Default|GetPercent) 0.3) (<= (Variables|Default|GetPercent) 0.4))
                    (bind _returnvalue_5 (Actor|GetActorOfClass "/Game/_GameManager/GameObjects/Treasure/Blueprint/BP_Treasure1.BP_Treasure1_C")))))))
          (else
            (Variables|Default|SetPercent (Math|Random|RandomFloat))
            (if (and (>= (Variables|Default|GetPercent) 0.4) (<= (Variables|Default|GetPercent) 1.0))
              (bind _returnvalue_6 (Actor|GetActorOfClass "/Game/_GameManager/GameObjects/Treasure/Blueprint/BP_Treasure1.BP_Treasure1_C"))
              (Variables|/Game/_GameManager/GameObjects/Treasure/Blueprint/BP_Treasure1.BP_Treasure1_C|SetTreasure%20Speed _returnvalue_6 8e+02)
              (Game|SpawnActorfromClass "/Game/_GameManager/GameObjects/Treasure/Blueprint/BP_Treasure1.BP_Treasure1_C" (Transformation|GetWorldTransform (Variables|Default|GetBox)) "Undefined" "MultiplyWithRoot" 0 0)
              (bind _returnvalue_7 (Actor|GetActorOfClass "/Game/_GameManager/GameObjects/Hook/Blueprint/BP_Hook.BP_Hook_C"))
              (Variables|/Game/_GameManager/GameObjects/Hook/Blueprint/BP_Hook.BP_Hook_C|SetIsMiddle? _returnvalue_7 true)
              (elif (and (>= (Variables|Default|GetPercent) 0.3) (<= (Variables|Default|GetPercent) 0.4))
                (bind _returnvalue_8 (Actor|GetActorOfClass "/Game/_GameManager/GameObjects/Treasure/Blueprint/BP_Treasure1.BP_Treasure1_C"))
                (Variables|/Game/_GameManager/GameObjects/Treasure/Blueprint/BP_Treasure1.BP_Treasure1_C|SetTreasure%20Speed _returnvalue_8 1e+03)
                (Game|SpawnActorfromClass "/Game/_GameManager/GameObjects/Treasure/Blueprint/BP_Treasure1.BP_Treasure1_C" (Transformation|GetWorldTransform (Variables|Default|GetBox)) "Undefined" "MultiplyWithRoot" 0 0)
                (bind _returnvalue_9 (Actor|GetActorOfClass "/Game/_GameManager/GameObjects/Hook/Blueprint/BP_Hook.BP_Hook_C"))
                (Variables|/Game/_GameManager/GameObjects/Hook/Blueprint/BP_Hook.BP_Hook_C|SetIsFast? _returnvalue_9 true)
                (elif (and (>= (Variables|Default|GetPercent) 0.0) (<= (Variables|Default|GetPercent) 0.3))
                  (bind _returnvalue_10 (Actor|GetActorOfClass "/Game/_GameManager/GameObjects/Treasure/Blueprint/BP_Treasure1.BP_Treasure1_C")))))))
        (else
          (goto _label_2)))
      (else
        (Variables|Default|SetPercent (Math|Random|RandomFloat))
        (if (and (>= (Variables|Default|GetPercent) 0.0) (<= (Variables|Default|GetPercent) 0.3))
          (bind _returnvalue_11 (Actor|GetActorOfClass "/Game/_GameManager/GameObjects/Treasure/Blueprint/BP_Treasure1.BP_Treasure1_C"))
          (Variables|/Game/_GameManager/GameObjects/Treasure/Blueprint/BP_Treasure1.BP_Treasure1_C|SetTreasure%20Speed _returnvalue_11 8e+02)
          (Game|SpawnActorfromClass "/Game/_GameManager/GameObjects/Treasure/Blueprint/BP_Treasure1.BP_Treasure1_C" (Transformation|GetWorldTransform (Variables|Default|GetBox)) "Undefined" "MultiplyWithRoot" 0 0)
          (bind _returnvalue_12 (Actor|GetActorOfClass "/Game/_GameManager/GameObjects/Hook/Blueprint/BP_Hook.BP_Hook_C"))
          (Variables|/Game/_GameManager/GameObjects/Hook/Blueprint/BP_Hook.BP_Hook_C|SetIsMiddle? _returnvalue_12 true)
          (elif (and (>= (Variables|Default|GetPercent) 0.3) (<= (Variables|Default|GetPercent) 0.4))
            (bind _returnvalue_13 (Actor|GetActorOfClass "/Game/_GameManager/GameObjects/Treasure/Blueprint/BP_Treasure1.BP_Treasure1_C"))
            (Variables|/Game/_GameManager/GameObjects/Treasure/Blueprint/BP_Treasure1.BP_Treasure1_C|SetTreasure%20Speed _returnvalue_13 1e+03)
            (Game|SpawnActorfromClass "/Game/_GameManager/GameObjects/Treasure/Blueprint/BP_Treasure1.BP_Treasure1_C" (Transformation|GetWorldTransform (Variables|Default|GetBox)) "Undefined" "MultiplyWithRoot" 0 0)
            (bind _returnvalue_14 (Actor|GetActorOfClass "/Game/_GameManager/GameObjects/Hook/Blueprint/BP_Hook.BP_Hook_C"))
            (Variables|/Game/_GameManager/GameObjects/Hook/Blueprint/BP_Hook.BP_Hook_C|SetIsFast? _returnvalue_14 true)
            (elif (and (>= (Variables|Default|GetPercent) 0.4) (<= (Variables|Default|GetPercent) 1.0))
              (bind _returnvalue_15 (Actor|GetActorOfClass "/Game/_GameManager/GameObjects/Treasure/Blueprint/BP_Treasure1.BP_Treasure1_C")))))))
    (else
      (goto _label))))

(event EventBeginPlay
  (Utilities|Time|SetTimerbyEvent (delegate Custom|Spawn) 5.0 true))

(fn ConstructionScript)
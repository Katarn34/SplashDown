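; Spawner that drops treasures or urchins (BP_Ursin) at its location, tracking count and last spawn type.
; Spawn is gated by game end, big-treasure appearance and a count cap, then picks one of three phases from HUD_Timer's clock.
; Two random rolls per phase choose treasure speed and urchin substitution, with urchin odds rising in later phases; most treasure spawns are delayed.
; The repeating-timer setup for Spawn is unwired here.
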(event Custom|Spawn
  (bind _bullespawnobjet (Variables|Default|GetBulleSpawnObjet))
  (bind _bullespawnobjet_2 (Variables|Default|GetBulleSpawnObjet))
  (bind _bullespawnobjet_3 (Variables|Default|GetBulleSpawnObjet))
  ;[1 1 1] First Minute
  (bind _returnvalue (Actor|GetActorOfClass "/Game/_GameManager/GameObjects/Big_Treasure/Blueprint/BP_SpawnBigTreasure.BP_SpawnBigTreasure_C"))
  (if (not (Variables|/Game/_GameManager/GameObjects/Big_Treasure/Blueprint/BP_SpawnBigTreasure.BP_SpawnBigTreasure_C|GetBig%20Treasure%20Appear _returnvalue))
    (if (not (Variables|Default|GetGame%20Finish))
      (if (<= (Variables|Default|GetCount) 4.0)
        (|Min/Seccondition
          (:else
            ;[1 1 1] Second minute
            (|2mincondition :!label _label
              (:else
                ;[1 1 1] Last Minute
                (|3emecondition :!label _label_2
                  (:else
                    (Variables|Default|SetPercent (Math|Random|RandomFloat))
                    (Variables|Default|SetPercentUrsins (Math|Random|RandomFloat))
                    (|PercentCondition
                      (:then
                        (goto _label_3 execute2))
                      (:then2
                        (goto _label_3 execute3))
                      (:then3
                        (|Ursincondition :!label _label_3
                          (:else
                            (Utilities|FlowControl|Delay 1.5)
                            (Components|Activation|SetAutoActivate _bullespawnobjet_3 false)
                            (Audio|PlaySound2D "/Game/Sound_Sam/SD/Enviro/SC_Spawn_de_tresor.SC_Spawn_de_tresor" 1.0 1.0 0.0 0 0)
                            (bind _returnvalue_2 (Game|SpawnActorfromClass "/Game/_GameManager/GameObjects/Treasure/Blueprint/BP_Treasure1.BP_Treasure1_C" (Math|Transform|MakeTransform (Transformation|GetWorldLocation (Variables|Default|GetDefaultSceneRoot)) "0, 0, 0" "1.000000,1.000000,1.000000") "Undefined" "MultiplyWithRoot" 0 0))
                            (Variables|/Game/_GameManager/GameObjects/Treasure/Blueprint/BP_Treasure1.BP_Treasure1_C|SetTreasure%20Speed _returnvalue_2 1e+03)
                            (Variables|Default|SetCount (+ (Variables|Default|GetCount) 1.0))
                            (Variables|Default|SetIsFast true))
                          (:else2
                            (Utilities|FlowControl|Delay 1.5)
                            (Components|Activation|SetAutoActivate _bullespawnobjet_3 false)
                            (Audio|PlaySound2D "/Game/Sound_Sam/SD/Enviro/SC_Spawn_de_tresor.SC_Spawn_de_tresor" 1.0 1.0 0.0 0 0)
                            (bind _returnvalue_3 (Game|SpawnActorfromClass "/Game/_GameManager/GameObjects/Treasure/Blueprint/BP_Treasure1.BP_Treasure1_C" (Math|Transform|MakeTransform (Transformation|GetWorldLocation (Variables|Default|GetDefaultSceneRoot)) "0, 0, 0" "1.000000,1.000000,1.000000") "Undefined" "MultiplyWithRoot" 0 0))
                            (Variables|/Game/_GameManager/GameObjects/Treasure/Blueprint/BP_Treasure1.BP_Treasure1_C|SetTreasure%20Speed _returnvalue_3 6e+02)
                            (Variables|Default|SetCount (+ (Variables|Default|GetCount) 1.0))
                            (Variables|Default|SetIsSlow true))
                          (:then
                            (CallFunction|Ursins :!label _label_4))
                          (:then2
                            (goto _label_4))
                          (:else3
                            (Utilities|FlowControl|Delay 1.5)
                            (Components|Activation|SetAutoActivate _bullespawnobjet_3 false)
                            (Audio|PlaySound2D "/Game/Sound_Sam/SD/Enviro/SC_Spawn_de_tresor.SC_Spawn_de_tresor" 1.0 1.0 0.0 0 0)
                            (bind _returnvalue_4 (Game|SpawnActorfromClass "/Game/_GameManager/GameObjects/Treasure/Blueprint/BP_Treasure1.BP_Treasure1_C" (Math|Transform|MakeTransform (Transformation|GetWorldLocation (Variables|Default|GetDefaultSceneRoot)) "0, 0, 0" "1.000000,1.000000,1.000000") "Undefined" "MultiplyWithRoot" 0 0))
                            (Variables|/Game/_GameManager/GameObjects/Treasure/Blueprint/BP_Treasure1.BP_Treasure1_C|SetTreasure%20Speed _returnvalue_4 8e+02)
                            (Variables|Default|SetCount (+ (Variables|Default|GetCount) 1.0))
                            (Variables|Default|SetIsMid true))
                          (:then3
                            (goto _label_4))))))))
              (:then
                (goto _label_2))
              (:else2
                (Variables|Default|SetPercent (Math|Random|RandomFloat))
                (Variables|Default|SetPercentUrsins (Math|Random|RandomFloat))
                (|CheckFast/Slow/mid
                  (:then
                    (goto _label_5 execute2))
                  (:then2
                    (goto _label_5 execute3))
                  (:then3
                    (|CheckUrsinsCondition :!label _label_5
                      (:else
                        (Utilities|FlowControl|Delay 1.5)
                        (Components|Activation|SetAutoActivate _bullespawnobjet_2 false)
                        (Audio|PlaySound2D "/Game/Sound_Sam/SD/Enviro/SC_Spawn_de_tresor.SC_Spawn_de_tresor" 1.0 1.0 0.0 0 0)
                        (bind _returnvalue_5 (Game|SpawnActorfromClass "/Game/_GameManager/GameObjects/Treasure/Blueprint/BP_Treasure1.BP_Treasure1_C" (Math|Transform|MakeTransform (Transformation|GetWorldLocation (Variables|Default|GetDefaultSceneRoot)) "0, 0, 0" "1.000000,1.000000,1.000000") "Undefined" "MultiplyWithRoot" 0 0))
                        (Variables|/Game/_GameManager/GameObjects/Treasure/Blueprint/BP_Treasure1.BP_Treasure1_C|SetTreasure%20Speed _returnvalue_5 1e+03)
                        (Variables|Default|SetCount (+ (Variables|Default|GetCount) 1.0))
                        (Variables|Default|SetIsFast true))
                      (:else2
                        (Utilities|FlowControl|Delay 1.5)
                        (Components|Activation|SetAutoActivate _bullespawnobjet_2 false)
                        (Audio|PlaySound2D "/Game/Sound_Sam/SD/Enviro/SC_Spawn_de_tresor.SC_Spawn_de_tresor" 1.0 1.0 0.0 0 0)
                        (bind _returnvalue_6 (Game|SpawnActorfromClass "/Game/_GameManager/GameObjects/Treasure/Blueprint/BP_Treasure1.BP_Treasure1_C" (Math|Transform|MakeTransform (Transformation|GetWorldLocation (Variables|Default|GetDefaultSceneRoot)) "0, 0, 0" "1.000000,1.000000,1.000000") "Undefined" "MultiplyWithRoot" 0 0))
                        (Variables|/Game/_GameManager/GameObjects/Treasure/Blueprint/BP_Treasure1.BP_Treasure1_C|SetTreasure%20Speed _returnvalue_6 6e+02)
                        (Variables|Default|SetCount (+ (Variables|Default|GetCount) 1.0))
                        (Variables|Default|SetIsSlow true))
                      (:then
                        (CallFunction|Ursins :!label _label_6))
                      (:then2
                        (goto _label_6))
                      (:else3
                        (Utilities|FlowControl|Delay 1.5)
                        (Components|Activation|SetAutoActivate _bullespawnobjet_2 false)
                        (Audio|PlaySound2D "/Game/Sound_Sam/SD/Enviro/SC_Spawn_de_tresor.SC_Spawn_de_tresor" 1.0 1.0 0.0 0 0)
                        (bind _returnvalue_7 (Game|SpawnActorfromClass "/Game/_GameManager/GameObjects/Treasure/Blueprint/BP_Treasure1.BP_Treasure1_C" (Math|Transform|MakeTransform (Transformation|GetWorldLocation (Variables|Default|GetDefaultSceneRoot)) "0, 0, 0" "1.000000,1.000000,1.000000") "Undefined" "MultiplyWithRoot" 0 0))
                        (Variables|/Game/_GameManager/GameObjects/Treasure/Blueprint/BP_Treasure1.BP_Treasure1_C|SetTreasure%20Speed _returnvalue_7 8e+02)
                        (Variables|Default|SetCount (+ (Variables|Default|GetCount) 1.0))
                        (Variables|Default|SetIsMid true))
                      (:then3
                        (goto _label_6))))))))
          (:then
            (goto _label))
          (:else2
            (Variables|Default|SetPercent (Math|Random|RandomFloat))
            (Variables|Default|SetPercentUrsins (Math|Random|RandomFloat))
            (|Percent1Condition
              (:then
                (|UrsinsCondition :!label _label_7
                  (:else
                    (Utilities|FlowControl|Delay 1.5)
                    (Components|Activation|Activate _bullespawnobjet false)
                    (Audio|PlaySound2D "/Game/Sound_Sam/SD/Enviro/SC_Spawn_de_tresor.SC_Spawn_de_tresor" 1.0 1.0 0.0 0 0)
                    (bind _returnvalue_8 (Game|SpawnActorfromClass "/Game/_GameManager/GameObjects/Treasure/Blueprint/BP_Treasure1.BP_Treasure1_C" (Math|Transform|MakeTransform (Transformation|GetWorldLocation (Variables|Default|GetDefaultSceneRoot)) "0, 0, 0" "1.000000,1.000000,1.000000") "Undefined" "MultiplyWithRoot" 0 0))
                    (Variables|/Game/_GameManager/GameObjects/Treasure/Blueprint/BP_Treasure1.BP_Treasure1_C|SetTreasure%20Speed _returnvalue_8 6e+02)
                    (Variables|Default|SetCount (+ (Variables|Default|GetCount) 1.0))
                    (Variables|Default|SetIsSlow true))
                  (:else2
                    (Utilities|FlowControl|Delay 1.5)
                    (Components|Activation|Activate _bullespawnobjet false)
                    (Audio|PlaySound2D "/Game/Sound_Sam/SD/Enviro/SC_Spawn_de_tresor.SC_Spawn_de_tresor" 1.0 1.0 0.0 0 0)
                    (bind _returnvalue_9 (Game|SpawnActorfromClass "/Game/_GameManager/GameObjects/Treasure/Blueprint/BP_Treasure1.BP_Treasure1_C" (Math|Transform|MakeTransform (Transformation|GetWorldLocation (Variables|Default|GetDefaultSceneRoot)) "0, 0, 0" "1.000000,1.000000,1.000000") "Undefined" "MultiplyWithRoot" 0 0))
                    (Variables|/Game/_GameManager/GameObjects/Treasure/Blueprint/BP_Treasure1.BP_Treasure1_C|SetTreasure%20Speed _returnvalue_9 8e+02)
                    (Variables|Default|SetCount (+ (Variables|Default|GetCount) 1.0))
                    (Variables|Default|SetIsMid true))
                  (:then
                    (CallFunction|Ursins :!label _label_8))
                  (:then2
                    (goto _label_8))
                  (:else3
                    (Audio|PlaySound2D "/Game/Sound_Sam/SD/Enviro/SC_Spawn_de_tresor.SC_Spawn_de_tresor" 1.0 1.0 0.0 0 0)
                    (bind _returnvalue_10 (Game|SpawnActorfromClass "/Game/_GameManager/GameObjects/Treasure/Blueprint/BP_Treasure1.BP_Treasure1_C" (Math|Transform|MakeTransform (Transformation|GetWorldLocation (Variables|Default|GetDefaultSceneRoot)) "0, 0, 0" "1.000000,1.000000,1.000000") "Undefined" "MultiplyWithRoot" 0 0))
                    (Variables|/Game/_GameManager/GameObjects/Treasure/Blueprint/BP_Treasure1.BP_Treasure1_C|SetTreasure%20Speed _returnvalue_10 1e+03)
                    (Variables|Default|SetCount (+ (Variables|Default|GetCount) 1.0))
                    (Variables|Default|SetIsFast true))
                  (:then3
                    (goto _label_8))))
              (:then2
                (goto _label_7 execute2))
              (:then3
                (goto _label_7 execute3)))))))))

(event Custom|Ursins
  ;[1 1 1] Spawn Ursins
  (Game|SpawnActorfromClass "/Game/_GameManager/GameObjects/Ursins/Blueprint/BP_Ursin.BP_Ursin_C" (Math|Transform|MakeTransform (Transformation|GetWorldLocation (Variables|Default|GetDefaultSceneRoot)) "0, 0, 0" "1.000000,1.000000,1.000000") "Undefined" "MultiplyWithRoot" 0 0)
  (Variables|Default|SetCount (+ (Variables|Default|GetCount) 1.0))
  (Variables|Default|SetIsUrsins true)
  (Variables|Default|SetIsFast false)
  (Variables|Default|SetIsSlow false)
  (Variables|Default|SetIsMid false))

(fn ConstructionScript)
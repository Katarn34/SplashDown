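; Spawner actor that places a BP_BigTreasure at its own location, with a spawn sound, whenever no big treasure is flagged as present.
; A looping timer set on BeginPlay is meant to poll the BigTreasureAppear flag and trigger a DoOnce-gated countdown while it is false.
; The countdown takes a longer delay the first time and a shorter one afterwards via Selection.
; Each spawn sets the flag and resets the gate.
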(event Custom|Big%20Treasure%20Spawn
  ;[1 1 1] Spawning System Big Treasure
  (Audio|PlaySound2D "/Game/Sound_Sam/SD/Enviro/SC_Spawn_de_gros_tresor.SC_Spawn_de_gros_tresor" 1.0 1.0 0.0 0 0)
  (Variables|Default|SetBig%20Treasure%20Appear true)
  (Game|SpawnActorfromClass "/Game/_GameManager/GameObjects/Big_Treasure/Blueprint/BP_BigTreasure.BP_BigTreasure_C" (Math|Transform|MakeTransform (.location (Transformation|GetActorTransform)) "0, 0, 0" "0.900000,0.900000,0.900000") "AdjustIfPossibleButAlwaysSpawn" "MultiplyWithRoot" 0 0)
  ;[1 1 1] Counting System
  (Utilities|FlowControl|DoOnce false) ; enters at Reset
)

(event Custom|Big%20Treasure%20Event%20Cooldown
  ;[1 1 1] Counting System
  (if (not (Variables|Default|GetBig%20Treasure%20Appear))
    (Utilities|FlowControl|DoOnce false
      (:Completed
        (switch int (Variables|Default|GetSelection)
          (:0
            (Utilities|FlowControl|Delay 6e+01)
            (CallFunction|BigTreasureSpawn)
            (Variables|Default|SetSelection 1))
          (:1
            (Utilities|FlowControl|Delay 3e+01)
            (CallFunction|BigTreasureSpawn)))))))

(event EventBeginPlay
  ;[1 1 1] Counting System
  (Utilities|Time|SetTimerbyEvent (delegate Custom|Big%20Treasure%20Event%20Cooldown) 0.1 true))

(fn ConstructionScript)
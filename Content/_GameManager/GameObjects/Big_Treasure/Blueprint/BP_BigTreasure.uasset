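; Big treasure chest actor that players catch with their hooks, bobbing in place through two timelines that loop from BeginPlay.
; BigTreasureFeedback rocks the mesh's pitch through four chained timelines, gated by a flag set after a short retriggerable delay.
; BigTreasureFinished clears SpawnWidget on player controllers, notifies any hook that hit it, destroys the chest and spawns a Niagara effect chosen by which hook won.
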(event Custom|Big%20Treasure%20Finished
  ;[1 1 1] When The Event is Finished, Execute "Big Treasure Hook Finished" and Destroy the Big Treasure
  (bind _outactors (Actor|GetAllActorsOfClass "/Game/Charaters/Player_Boat/Blueprint/BP_Player.BP_Player_C"))
  (for _array_element _outactors
    (bind _outactors_2 (Actor|GetAllActorsOfClass "/Game/_GameManager/Controller/BP_PlayerController.BP_PlayerController_C"))
    (for _array_element_2 _outactors_2
      (Variables|/Game/_GameManager/Controller/BP_PlayerController.BP_PlayerController_C|SetSpawn%20Widget%20? _array_element_2 false)
      (if (Variables|/Game/_GameManager/GameObjects/Hook/Blueprint/BP_Hook.BP_Hook_C|GetBig%20Treasure%20Hit (.AsBP%20Hook (Utilities|Casting|CastToBP_Hook (Variables|/Script/Engine.ChildActorComponent|GetChildActor (Variables|/Game/Charaters/Player_Boat/Blueprint/BP_Player.BP_Player_C|GetChildActor _array_element)))))
        (Default|BigTreasureHookFinished (.AsBP%20Hook (Utilities|Casting|CastToBP_Hook (Variables|/Script/Engine.ChildActorComponent|GetChildActor (Variables|/Game/Charaters/Player_Boat/Blueprint/BP_Player.BP_Player_C|GetChildActor _array_element)))))
        (Default|HitTreasure/Ursin (.AsBP%20Hook (Utilities|Casting|CastToBP_Hook (Variables|/Script/Engine.ChildActorComponent|GetChildActor (Variables|/Game/Charaters/Player_Boat/Blueprint/BP_Player.BP_Player_C|GetChildActor _array_element)))))
        (Utilities|IsValid self
          (:Is%20Valid
            (Actor|DestroyActor)
            (bind _outactors_3 (Actor|GetAllActorsOfClass "/Game/_GameManager/GameObjects/Hook/Blueprint/BP_Hook.BP_Hook_C"))
            (if (Variables|/Game/_GameManager/GameObjects/Hook/Blueprint/BP_Hook.BP_Hook_C|GetWinner (Utilities|Array|Get(acopy) _outactors_3))
              (Niagara|SpawnSystematLocation "/Game/VFX/Effects/AgoraNeon/NS_NeonAgoraOr.NS_NeonAgoraOr" "440.000000,250.000000,400.000000" "90.000000,0.000000,0.000000")
              (elif (Variables|/Game/_GameManager/GameObjects/Hook/Blueprint/BP_Hook.BP_Hook_C|GetWinner (Utilities|Array|Get(acopy) _outactors_3 1))
                (Niagara|SpawnSystematLocation "/Game/VFX/Effects/AgoraNeon/NS_NeonAgora.NS_NeonAgora" "440.000000,250.000000,400.000000" "90.000000,0.000000,0.000000")))))))))

(event Custom|Big%20Treasure%20Feedback
  (Utilities|FlowControl|Sequence
    (:then_0
      (Utilities|FlowControl|RetriggerableDelay 0.2)
      (Variables|Default|SetCan%20go%20Next%20Animation%20? true))
    (:then_1
      (bind _rotating_movemnt (Timeline|Rotating%20Chest PlayFromStart)
        (:Update
          (Transformation|SetRelativeRotation (Variables|Default|GetBig%20Treasure%20Mesh) (Math|Rotator|MakeRotator 0.0 _rotating_movemnt 9e+01) false false))
        (:Finished
          (if (Variables|Default|GetCan%20go%20Next%20Animation%20?)
            (bind _rotating_movemnt_2 (Timeline|Rotating%20Chest%20Reverse ReverseFromEnd)
              (:Update
                (Transformation|SetRelativeRotation (Variables|Default|GetBig%20Treasure%20Mesh) (Math|Rotator|MakeRotator 0.0 _rotating_movemnt_2 9e+01) false false))
              (:Finished
                (if (Variables|Default|GetCan%20go%20Next%20Animation%20?)
                  (bind _rotating_movemnt_3 (Timeline|Timeline PlayFromStart)
                    (:Update
                      (Transformation|SetRelativeRotation (Variables|Default|GetBig%20Treasure%20Mesh) (Math|Rotator|MakeRotator 0.0 _rotating_movemnt_3 9e+01) false false))
                    (:Finished
                      (if (Variables|Default|GetCan%20go%20Next%20Animation%20?)
                        (bind _rotating_movemnt_4 (Timeline|Timeline_0 ReverseFromEnd)
                          (:Update
                            (Transformation|SetRelativeRotation (Variables|Default|GetBig%20Treasure%20Mesh) (Math|Rotator|MakeRotator 0.0 _rotating_movemnt_4 9e+01) false false)))))))))))))))

(event EventBeginPlay
  ;[1 1 1] Floating movement of the big Treasure
  (bind _z_axis_movement (Timeline|Floating%20Object Play)
    (:Update
      (Transformation|SetRelativeLocation (Variables|Default|GetBig%20Treasure%20Mesh) _z_axis_movement false false))
    (:Finished
      (bind _z_axis_movement_2 (Timeline|Reverse%20Floating%20Object ReverseFromEnd)
        (:Update
          (Transformation|SetRelativeLocation (Variables|Default|GetBig%20Treasure%20Mesh) _z_axis_movement_2 false false))
        (:Finished
          (Timeline|Floating%20Object PlayFromStart))))))

(fn ConstructionScript)
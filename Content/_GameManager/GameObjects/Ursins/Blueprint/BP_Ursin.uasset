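; BP_Ursin is a physics-driven urchin object that launches with an impulse on spawn and destroys itself after a delay unless StopDestroy is set.
; Above a height threshold, Tick adds downward velocity that grows with the excess height and mass scale.
; Hits ignore BP_Hook, bounce off BP_Treasure1 upward and along Y according to current Y velocity, and otherwise add a small impulse to maintain height.
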(event EventBeginPlay
  ;[1 1 1] Base Impulse
  (Variables|/Script/Engine.ProjectileMovementComponent|SetInitialSpeed (Variables|Default|GetProjectileMovement) (Variables|Default|GetTreasure%20Speed))
  (Physics|AddImpulse (Variables|Default|GetUrsin) (Variables|Default|GetFirst%20Impulse) "None" true)
  (Utilities|FlowControl|Delay 15.0)
  (if (not (Variables|Default|GetStop%20Destroy))
    (Actor|DestroyActor)))

(event EventTick
  (params (DeltaSeconds :type Float%20%28single-precision%29))
  (bind _returnvalue (Transformation|GetActorLocation))
  (if (> (.z _returnvalue) (Variables|Default|GetHeight%20Threshold))
    (Class|PrimitiveComponent|SetAllPhysicsLinearVelocity (Variables|Default|GetUrsin) (Math|Vector|MakeVector 0.0 0.0 (* DeltaSeconds (Variables|Default|GetAppliedForce) (Class|PrimitiveComponent|GetMassScale (Variables|Default|GetUrsin) "None") -1.0 (- (.z _returnvalue) (Variables|Default|GetHeight%20Threshold)))) true)))

(event Collision|EventHit
  (params (MyComp :type Primitive%20Component%20Object%20Reference) (Other :type Actor%20Object%20Reference) (OtherComp :type Primitive%20Component%20Object%20Reference) (bSelfMoved :type Boolean) (HitLocation :type Vector :default "0, 0, 0") (HitNormal :type Vector :default "0, 0, 0") (NormalImpulse :type Vector :default "0, 0, 0") (Hit :type Hit%20Result%20Structure%20%28by%20ref%29))
  ;[1 1 1] What is the treasure touching verification
  (bind _asbp_hook (Utilities|Casting|CastToBP_Hook Other)
    (:then
      _)
    (:CastFailed
      _))
  (if (not (== _asbp_hook Other))
    (bind _asbp_treasure_1 (Utilities|Casting|CastToBP_Treasure1 Other)
      (:then
        _)
      (:CastFailed
        _))
    (if (== Other _asbp_treasure_1)
      ;[1 1 1] Add impulse on touching itself on linear velocity check
      (bind _returnvalue (Physics|GetPhysicsLinearVelocity (Variables|Default|GetUrsin) "None"))
      (if (<= (.y _returnvalue) 1.0)
        (Physics|AddImpulse (Variables|Default|GetUrsin) "0.000000,-10.000000,5.000000" "None" true)
        (else
          (Physics|AddImpulse (Variables|Default|GetUrsin) "0.000000,10.000000,5.000000" "None" true)))
      (else
        ;[1 1 1] Add Impulse to maintain height
        (Physics|AddImpulse (Variables|Default|GetUrsin) "0.000000,0.100000,0.100000" "None" false)))))

(fn ConstructionScript
  (Transformation|SetActorRotation "0.000000,90.000000,0.000000"))
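; Game mode for a local two-player submarine treasure game, creating the second player, spawning and possessing both pawns, coloring subs and hooks orange and green, and starting music.
; A one-second timer spawns treasures or urchins at random spawners while under five exist and no big treasure appears.
; Urchins unlock after 30 seconds and are limited to two.
; SaveScore adds HUD scores and entered names to a sorted, top-three save-slot leaderboard.
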(event Custom|Stop%20Playing%20Sound%20Composition
  ;[1 1 1] Stop playing sound compo custom event
  (Utilities|IsValid (stale EventBeginPlay _returnvalue_2)
    (:Is%20Valid
      (Audio|Components|Audio|Stop (stale EventBeginPlay _returnvalue_2)))))

(event Custom|Spawnn
  ;[1 1 1] Spawner
  (bind _outactors (Actor|GetAllActorsOfClass "/Game/_GameManager/GameObjects/Treasure/Blueprint/BP_Treasure1.BP_Treasure1_C"))
  (bind _outactors_2 (Actor|GetAllActorsOfClass "/Game/_GameManager/GameObjects/Ursins/Blueprint/BP_Ursin.BP_Ursin_C"))
  (if (< (+ (Utilities|Array|Length _outactors_2) (Utilities|Array|Length _outactors)) 5)
    (bind _returnvalue (Actor|GetActorOfClass "/Game/_GameManager/GameObjects/Big_Treasure/Blueprint/BP_SpawnBigTreasure.BP_SpawnBigTreasure_C"))
    (if (not (Variables|/Game/_GameManager/GameObjects/Big_Treasure/Blueprint/BP_SpawnBigTreasure.BP_SpawnBigTreasure_C|GetBig%20Treasure%20Appear _returnvalue))
      (if (not (Variables|Default|GetSpawned?))
        (Variables|Default|SetSpawned? true)
        (Variables|Default|SetRandom%20Spawner%20Choosed (Utilities|Array|MakeArray (.OutItem (Utilities|Array|Random (Variables|Default|GetSpawn)))))
        (Components|Activation|Activate (Variables|/Game/_GameManager/GameObjects/Spawner/BP_Spawne.BP_Spawne_C|GetBulleSpawnObjet (Utilities|Array|Get(acopy) (Variables|Default|GetRandom%20Spawner%20Choosed))) true)
        (Utilities|FlowControl|Delay 1.5)
        (if (>= (Math|Random|RandomFloat) 0.3)
          (Game|SpawnActorfromClass "/Game/_GameManager/GameObjects/Treasure/Blueprint/BP_Treasure1.BP_Treasure1_C" (Math|Transform|MakeTransform (Transformation|GetActorLocation (Utilities|Array|Get(acopy) (Variables|Default|GetRandom%20Spawner%20Choosed))) "0, 0, 0" "1.000000,1.000000,1.000000") "AdjustIfPossibleButAlwaysSpawn" "MultiplyWithRoot" 0 0 :!label _label)
          (else
            (bind _outactors_3 (Actor|GetAllActorsOfClass "/Game/_GameManager/GameObjects/Ursins/Blueprint/BP_Ursin.BP_Ursin_C"))
            (if (>= (Utilities|Array|Length _outactors_3) 2)
              (goto _label)
              (elif (Variables|Default|GetUrsin%20Can%20Spawn%20?)
                (Game|SpawnActorfromClass "/Game/_GameManager/GameObjects/Ursins/Blueprint/BP_Ursin.BP_Ursin_C" (Math|Transform|MakeTransform (Transformation|GetActorLocation (Utilities|Array|Get(acopy) (Variables|Default|GetRandom%20Spawner%20Choosed))) "0, 0, 0" "1.000000,1.000000,1.000000") "AdjustIfPossibleButAlwaysSpawn" "MultiplyWithRoot" 0 0)
                (else
                  (goto _label))))))
        (Audio|PlaySound2D "/Game/Sound_Sam/SD/Enviro/SC_Spawn_de_tresor.SC_Spawn_de_tresor" 1.0 1.0 0.0 0 0)
        (Utilities|Array|Clear (Variables|Default|GetRandom%20Spawner%20Choosed))
        (Variables|Default|SetSpawned? false)))))

(event Custom|BeginMatch
  (bind _outactors (Actor|GetAllActorsOfClass "/Script/Engine.PlayerStart"))
  (Variables|Default|SetPlayer%20Start _outactors)
  (for (_array_element _array_index) (Variables|Default|GetPlayer%20Controllers)
    (bind _returnvalue (Game|SpawnActorfromClass "/Game/Charaters/Player_Boat/Blueprint/BP_Player.BP_Player_C" (Transformation|GetActorTransform (Utilities|Array|Get(acopy) (Variables|Default|GetPlayer%20Start) _array_index)) "AdjustIfPossibleButAlwaysSpawn" "MultiplyWithRoot" 0 _array_index 0))
    (Pawn|Possess _array_element _returnvalue)
    (Input|SetInputModeGameOnly _array_element false)))

(event Custom|Save%20Score
  (bind _save_ref (Variables|Default|GetSave%20Ref))
  (bind _asbp_save_final (Utilities|Casting|CastToBP_SaveFinal _save_ref))
  (CallFunction|Load/SaveGame (Variables|Default|GetSlot%20Save))
  (bind _foundwidgets (Widget|GetAllWidgetsOfClass "/Game/UI-UX/HUD/HUD_Score.HUD_Score_C" true))
  (for _array_element _foundwidgets
    (for (_array_element_2 _array_index) (Utilities|Array|MakeArray (Variables|/Game/UI-UX/HUD/HUD_Score.HUD_Score_C|GetScoreJ1 _array_element) (Variables|/Game/UI-UX/HUD/HUD_Score.HUD_Score_C|GetScoreJ2 _array_element))
      (switch int _array_index
        (:0
          (bind _foundwidgets_2 (Widget|GetAllWidgetsOfClass "/Game/UI-UX/Menus/WBP_ChooseName.WBP_ChooseName_C" true))
          (Variables|Default|SetName (Variables|/Game/UI-UX/Menus/WBP_ChooseName.WBP_ChooseName_C|GetName_Joueur%201 (Utilities|Array|Get(acopy) _foundwidgets_2))))
        (:1
          (bind _foundwidgets_3 (Widget|GetAllWidgetsOfClass "/Game/UI-UX/Menus/WBP_ChooseName.WBP_ChooseName_C" true))
          (Variables|Default|SetName (Variables|/Game/UI-UX/Menus/WBP_ChooseName.WBP_ChooseName_C|GetName_Joueur2 (Utilities|Array|Get(acopy) _foundwidgets_3)))))
      (Utilities|Array|Add (Variables|/Game/UI-UX/Menus/Save_Game/BP_SaveFinal.BP_SaveFinal_C|GetScore _asbp_save_final) (Utilities|Struct|MakeStruct_Scores _array_element_2 (Variables|Default|GetName)))
      (Variables|/Game/UI-UX/Menus/Save_Game/BP_SaveFinal.BP_SaveFinal_C|SetScore _asbp_save_final (Variables|/Game/UI-UX/Menus/Save_Game/BP_SaveFinal.BP_SaveFinal_C|GetScore _asbp_save_final)))
    (for _array_element_3 (Variables|/Game/UI-UX/Menus/Save_Game/BP_SaveFinal.BP_SaveFinal_C|GetScore _asbp_save_final)
      (bind _sorted_array (CallFunction|Sort (Variables|/Game/UI-UX/Menus/Save_Game/BP_SaveFinal.BP_SaveFinal_C|GetScore _asbp_save_final))))
    (Utilities|Array|Resize _sorted_array 3)
    (bind _asbp_save_final_2 (Utilities|Casting|CastToBP_SaveFinal (Variables|Default|GetSave%20Ref)))
    (Variables|/Game/UI-UX/Menus/Save_Game/BP_SaveFinal.BP_SaveFinal_C|SetScore _asbp_save_final_2 _sorted_array)
    (SaveGame|SaveGametoSlot (Variables|Default|GetSave%20Ref) (Variables|Default|GetSlot%20Save))))

(event Custom|Ursin%20Spawn
  (Variables|Default|SetUrsin%20Can%20Spawn%20? true))

(event EventBeginPlay
  (Utilities|Time|SetTimerbyEvent (delegate Custom|Ursin%20Spawn) 3e+01)
  (Utilities|FlowControl|Sequence
    (:then_0
      (if (not (>= (Utilities|Array|Length (Variables|Default|GetPlayer%20Controllers)) 2))
        (bind _returnvalue (Class|GameplayStatics|CreatePlayer -1))
        ;[1 1 1] à remettre pour faire marcher les 2 mannettes
        (Input|AddMappingContext (PlayerController|LocalPlayerSubsystems|GetEnhancedInputLocalPlayerSubsystem _returnvalue) "/Game/_GameManager/Input/IMC_Player.IMC_Player" 0 "(bIgnoreAllPressedKeysUntilRelease=True,bForceImmediately=False,bNotifyUserSettings=False)")))
    (:then_1
      ;[1 1 1] Spawner
      (CallFunction|BeginMatch)
      (bind _outactors (Actor|GetAllActorsOfClass "/Game/_GameManager/GameObjects/Spawner/BP_Spawne.BP_Spawne_C"))
      (Variables|Default|SetSpawn _outactors)
      (Utilities|Time|SetTimerbyEvent (delegate Custom|Spawnn) 1.0 true)
      ;[1 1 1] Changing Boats Material
      (|CollapseGraph)
      ;[1 1 1] Playing sound Composition
      (bind _returnvalue_2 (Audio|SpawnSound2D "/Game/Sound_Sam/SD/Compo/SC_compo_sam.SC_compo_sam" 1.0 1.0 0.0 0)))))

(event EventHandleStartingNewPlayer
  (params (NewPlayer :type Player%20Controller%20Object%20Reference))
  (Utilities|Array|AddUnique (Variables|Default|GetPlayer%20Controllers) NewPlayer))

(fn ConstructionScript)

(fn Sort
  (params (Score :type Array%20of%20Struct%20Scores%20Structures))
  (bind _returnvalue (Utilities|Array|LastIndex Score))
  (for _index (range 0 _returnvalue)
    (bind _output_get (LocalVariables|SetMin%20Index _index))
    (for _index_2 (range (+ _output_get 1) _returnvalue)
      (Development|PrintString (Utilities|String|ToString(Integer) (.Score (Utilities|Struct|BreakStruct_Scores (Utilities|Array|Get(acopy) Score _index_2)))))
      (if (> (.Score (Utilities|Struct|BreakStruct_Scores (Utilities|Array|Get(acopy) Score _index_2))) (.Score (Utilities|Struct|BreakStruct_Scores (Utilities|Array|Get(acopy) Score (LocalVariables|GetMin%20Index)))))
        (LocalVariables|SetMin%20Index _index_2)))
    (if (!= _index (LocalVariables|GetMin%20Index))
      (Utilities|Array|Swap Score _index (LocalVariables|GetMin%20Index))
      (return Score))))

(fn Load/SaveGame
  (params (SlotName :type String))
  (bind _returnvalue (SaveGame|DoesSaveGameExist SlotName))
  (if _returnvalue
    (bind _returnvalue_2 (SaveGame|LoadGamefromSlot SlotName))
    (Variables|Default|SetSave%20Ref _returnvalue_2)
    (else
      (bind _returnvalue_3 (SaveGame|CreateSaveGameObject "/Game/UI-UX/Menus/Save_Game/BP_SaveFinal.BP_SaveFinal_C"))
      (bind _output_get (Variables|Default|SetSave%20Ref _returnvalue_3))))
  (Utilities|Casting|CastToBP_SaveFinal _output_get)
  (SaveGame|SaveGametoSlot (Variables|Default|GetSave%20Ref) (Variables|Default|GetSlot%20Save))
  (return (Variables|Default|GetSave%20Ref)))
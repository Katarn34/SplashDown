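; Player boat Blueprint that handles a button-mash input for the big treasure event, alongside a game timer event.
; While BigTreasuresAppear is set, each A press finds the top-level HUD_Spam widgets, increments the first one's Count and calls Spam on them, with debug prints.
; The Timer0 event switches the player controller to UI-only input and shows the mouse cursor.
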(event Custom|Timer0
  (bind _returnvalue (Game|GetPlayerController 0))
  ;[1 1 1] Timer
  (Input|SetInputModeUIOnly _returnvalue 0 "DoNotLock" false)
  (Variables|/Script/Engine.PlayerController|SetbShowMouseCursor _returnvalue true))

(event Input|KeyboardEvents|A
  (params (Key :type Key%20Structure))
  ;[1 1 1] Spam
  (:Pressed
    (Development|PrintString "Hello")
    (if (Variables|Default|GetBigTreasuresAppear)
      (bind _foundwidgets (Widget|GetAllWidgetsOfClass "/Game/UI-UX/HUD/HUD_Spam.HUD_Spam_C" true))
      (bind _output_get (Variables|/Game/UI-UX/HUD/HUD_Spam.HUD_Spam_C|SetCount (Utilities|Array|Get(acopy) _foundwidgets) (+ (Variables|/Game/UI-UX/HUD/HUD_Spam.HUD_Spam_C|GetCount (Utilities|Array|Get(acopy) _foundwidgets)) 1.0)))
      (Default|Spam _foundwidgets)
      (Development|PrintString (Utilities|String|ToString(Float) _output_get)))))

(fn ConstructionScript)